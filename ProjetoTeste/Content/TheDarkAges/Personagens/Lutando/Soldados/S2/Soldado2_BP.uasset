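; Soldier 2 character Blueprint that acts out a scripted, endlessly repeating fight animation, with no input, AI or combat logic.
; After an initial delay on BeginPlay, it plays block, two attack and damage (Dano) montages in sequence, using each returned montage length as the next delay.
; It sets an Idle2 flag during the attack-to-damage stretch, clears it afterwards, then wires back to the block after a short pause.
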(event EventBeginPlay
  (Utilities|FlowControl|Delay 5.25)
  (bind _returnvalue (Animation|PlayAnimMontage "/Game/TheDarkAges/Personagens/Lutando/Soldados/S2/S2_Block.S2_Block" 1.0 "None" :!label _label))
  (Utilities|FlowControl|Delay _returnvalue)
  (bind _returnvalue_2 (Animation|PlayAnimMontage "/Game/TheDarkAges/Personagens/Lutando/Soldados/S2/S2_Attack1.S2_Attack1" 1.0 "None"))
  (Variables|Default|SetIdle2 true)
  (Utilities|FlowControl|Delay _returnvalue_2)
  (bind _returnvalue_3 (Animation|PlayAnimMontage "/Game/TheDarkAges/Personagens/Lutando/Soldados/S2/S2_Attack2.S2_Attack2" 1.0 "None"))
  (Utilities|FlowControl|Delay _returnvalue_3)
  (Utilities|FlowControl|Delay 1.0)
  (bind _returnvalue_4 (Animation|PlayAnimMontage "/Game/TheDarkAges/Personagens/Lutando/Soldados/S2/S2_Dano.S2_Dano" 1.0 "None"))
  (Utilities|FlowControl|Delay _returnvalue_4)
  (Variables|Default|SetIdle2 false)
  (Utilities|FlowControl|Delay 0.3)
  (goto _label))

(fn ConstructionScript)