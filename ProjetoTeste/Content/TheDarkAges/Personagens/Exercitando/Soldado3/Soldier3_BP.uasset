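; Soldier3_BP is a soldier character that performs a looping training routine as soon as play begins.
; BeginPlay plays a fixed sequence of training montages, repeating some of them, with hard-coded delays spacing each one.
; After the last delay the chain wires back to the first montage, so the routine runs endlessly without reacting to gameplay or montage completion.
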(event EventBeginPlay
  (Animation|PlayAnimMontage "/Game/TheDarkAges/Personagens/Exercitando/Soldado3/S3_treino1.S3_treino1" 1.0 "None" :!label _label)
  (Utilities|FlowControl|Delay 2.2)
  (Animation|PlayAnimMontage "/Game/TheDarkAges/Personagens/Exercitando/Soldado3/S3_Treino2.S3_Treino2" 1.0 "None")
  (Utilities|FlowControl|Delay 1.133)
  (Animation|PlayAnimMontage "/Game/TheDarkAges/Personagens/Exercitando/Soldado3/S3_Treino2.S3_Treino2" 1.0 "None")
  (Utilities|FlowControl|Delay 1.133)
  (Animation|PlayAnimMontage "/Game/TheDarkAges/Personagens/Exercitando/Soldado3/S3_Treino2.S3_Treino2" 1.0 "None")
  (Utilities|FlowControl|Delay 1.133)
  (Animation|PlayAnimMontage "/Game/TheDarkAges/Personagens/Exercitando/Soldado3/S3_Treino2.S3_Treino2" 1.0 "None")
  (Utilities|FlowControl|Delay 1.133)
  (Animation|PlayAnimMontage "/Game/TheDarkAges/Personagens/Exercitando/Soldado3/S3_Treino2.S3_Treino2" 1.0 "None")
  (Utilities|FlowControl|Delay 1.133)
  (Animation|PlayAnimMontage "/Game/TheDarkAges/Personagens/Exercitando/Soldado3/S3_Treino2.S3_Treino2" 1.0 "None")
  (Utilities|FlowControl|Delay 1.133)
  (Animation|PlayAnimMontage "/Game/TheDarkAges/Personagens/Exercitando/Soldado3/S3_Treino2_2.S3_Treino2_2" 1.0 "None")
  (Utilities|FlowControl|Delay 3.433)
  (Animation|PlayAnimMontage "/Game/TheDarkAges/Personagens/Exercitando/Soldado3/S3_Treino2_2.S3_Treino2_2" 1.0 "None")
  (Utilities|FlowControl|Delay 3.433)
  (Animation|PlayAnimMontage "/Game/TheDarkAges/Personagens/Exercitando/Soldado3/S3_Treino3.S3_Treino3" 1.0 "None")
  (Utilities|FlowControl|Delay 2.7)
  (goto _label))

(fn ConstructionScript)